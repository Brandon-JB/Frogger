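; Car actor that moves by projectile movement and acts as a hazard to the third-person character.
; When the movement component activates, it sets its initial and maximum speeds to random values between MinSpeed and MaxSpeed.
; Overlapping the character opens the MainGame level, while overlapping anything else destroys the car, with a debug print when the other actor is also a car.
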(event `self.ProjectileMovement.OnComponentActivated`
  (params (Component :type "ActorComponent Object Reference") (bReset :type Boolean))
  (bind _projectilemovement (`self.ProjectileMovement`))
  (bind _returnvalue (`KismetMathLibrary.RandomFloatInRange` (`self.MinSpeed`) (`self.MaxSpeed`)))
  (set `ProjectileMovementComponent.InitialSpeed` _returnvalue _projectilemovement)
  (set `ProjectileMovementComponent.MaxSpeed` _returnvalue _projectilemovement))

(event `self.ReceiveActorBeginOverlap`
  (params (OtherActor :type "Actor Object Reference"))
  (bind _returnvalue (`GameplayStatics.GetObjectClass` OtherActor))
  (if (`KismetMathLibrary.ClassIsChildOf` _returnvalue "/Game/ThirdPerson/Blueprints/BP_ThirdPersonCharacter.BP_ThirdPersonCharacter_C")
    (`GameplayStatics.OpenLevelBySoftObjectPtr` "/Game/Levels/MainGame.MainGame")
    (elif (`KismetMathLibrary.ClassIsChildOf` _returnvalue "Car_BP_C")
      (`KismetSystemLibrary.PrintString` "cra crah")
      (`self.K2_DestroyActor`)
      (else
        (`self.K2_DestroyActor`)))))

(fn `UserConstructionScript`)