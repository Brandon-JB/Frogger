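; CarSpawner_BP is a traffic spawner that periodically creates Car_BP actors at its TrafficSpawner component.
; Tick accumulates delta time until it reaches TimeBetweenSpawn, then resets the timer.
; Each interval rolls a random integer for an even chance of spawning a car at that component's world transform, so traffic arrives with irregular gaps.
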(event `self.ReceiveTick`
  (params (DeltaSeconds :type "Float (single-precision)"))
  (bind _output_get (set `self.TimeSinceSpawn` (+ DeltaSeconds (`self.TimeSinceSpawn`))))
  (if (>= _output_get (`self.TimeBetweenSpawn`))
    (set `self.TimeSinceSpawn` 0.0)
    (if (<= (`KismetMathLibrary.RandomIntegerInRange` 1 10) 5)
      (`|SpawnActorFromClass` "/Game/Blueprints/Car_BP.Car_BP_C" (`SceneComponent.K2_GetComponentToWorld` (`self.TrafficSpawner`)) "Undefined" "MultiplyWithRoot" null null))))

(fn `UserConstructionScript`)