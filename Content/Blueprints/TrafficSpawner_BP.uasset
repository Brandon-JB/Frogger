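; TrafficSpawner_BP is a spawner actor that periodically creates Traffic_BP actors at its TrafficSpawner component's world transform.
; On BeginPlay it waits a short delay, then spawns the first vehicle.
; Tick accumulates elapsed time and spawns another whenever it reaches TimeBetweenSpawn, then resets the timer.
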(event `self.ReceiveTick`
  (params (DeltaSeconds :type "Float (single-precision)"))
  (bind _output_get (set `self.TimeSinceSpawn` (+ DeltaSeconds (`self.TimeSinceSpawn`))))
  (if (>= _output_get (`self.TimeBetweenSpawn`))
    (set `self.TimeSinceSpawn` 0.0)
    (`|SpawnActorFromClass` "/Game/Blueprints/Traffic_BP.Traffic_BP_C" (`SceneComponent.K2_GetComponentToWorld` (`self.TrafficSpawner`)) "Undefined" "MultiplyWithRoot" null null)))

(event `self.ReceiveBeginPlay`
  (`KismetSystemLibrary.Delay` 1.0)
  (`|SpawnActorFromClass` "/Game/Blueprints/Traffic_BP.Traffic_BP_C" (`SceneComponent.K2_GetComponentToWorld` (`self.TrafficSpawner`)) "Undefined" "MultiplyWithRoot" null null))

(fn `UserConstructionScript`)