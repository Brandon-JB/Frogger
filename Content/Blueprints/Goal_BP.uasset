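; Goal pickup actor that ends the game with a win when the third-person character touches it.
; Tick spins the root by a fixed, frame-rate-dependent step, while a timeline started on BeginPlay feeds its track into a per-update actor offset for animated movement.
; On overlap, it checks the other actor's class against BP_ThirdPersonCharacter, prints a win message and opens YouWinLevel.
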(event `self.ReceiveTick`
  (params (DeltaSeconds :type "Float (single-precision)"))
  (`SceneComponent.K2_AddLocalRotation` (`self.DefaultSceneRoot`) (struct :`Yaw` 3.0) false false))

(event `self.ReceiveBeginPlay`
  (bind (_direction _newtrack_0) (`Timeline|Animation`)
    (:`Update`
      (`self.K2_AddActorLocalOffset` _newtrack_0))))

(event `self.ReceiveActorBeginOverlap`
  (params (OtherActor :type "Actor Object Reference"))
  (if (`KismetMathLibrary.ClassIsChildOf` (`GameplayStatics.GetObjectClass` OtherActor) "/Game/ThirdPerson/Blueprints/BP_ThirdPersonCharacter.BP_ThirdPersonCharacter_C")
    (`KismetSystemLibrary.PrintString` "Win")
    (`GameplayStatics.OpenLevelBySoftObjectPtr` "/Game/UI/YouWinLevel.YouWinLevel")))

(fn `UserConstructionScript`)